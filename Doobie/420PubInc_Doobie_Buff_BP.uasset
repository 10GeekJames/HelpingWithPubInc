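; Doobie buff for ARK that temporarily changes the player's hair and spreads on contact.
; On start, the server saves head and facial hair, forces a full-grown style and sets Weight to 1200.
; Its overlap sphere gives the buff to players lacking it, deactivating their Contagious_Buff, and teleports wild dinos upward, flipped over.
; Destruction restores the saved hair, but the Weight restore is never run.
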(event OnComponentBeginOverlap(OverlapSphere)
  (params (OtherActor :type Actor%20Object%20Reference) (OtherComp :type Primitive%20Component%20Object%20Reference) (OtherBodyIndex :type Integer) (bFromSweep :type Boolean) (SweepResult :type Hit%20Result%20Structure%20%28by%20ref%29))
  (Utilities|FlowControl|Sequence
    (:then_0
      (bind _asshootercharacter (Utilities|Casting|CastToShooterCharacter OtherActor))
      (bind _returnvalue (Class|PrimalCharacter|HasBuff _asshootercharacter "420PubInc_Doobie_Buff_BP_C" false))
      (if (not _returnvalue)
        (Utilities|FlowControl|Sequence
          (:then_0
            (Class|PrimalBuff|StaticAddBuff "420PubInc_Doobie_Buff_BP_C" _asshootercharacter 0 0 false))
          (:then_1
            (bind _returnvalue_2 (Class|PrimalCharacter|GetBuff _asshootercharacter "/Game/Mods/420PubInc/Contagious_Buff.Contagious_Buff_C"))
            (Class|PrimalBuff|BPDeactivate _returnvalue_2)
            (Class|PrimalBuff|StaticAddBuff "420PubInc_Doobie_Buff_BP_C" _asshootercharacter 0 0 false)))))
    (:then_1
      (bind _asdino_character_bp_c (Utilities|Casting|CastToDino_Character_BP OtherActor))
      (if (Class|PrimalCharacter|IsWildSlow _asdino_character_bp_c)
        (Transformation|Teleport _asdino_character_bp_c (+ (Transformation|GetActorLocation _asdino_character_bp_c) "0.000000,0.000000,840.000000") "0.000000, 0,180.000000")))))

(event EventEndPlay
  (params (EndPlayReason :type EEndPlayReason%20Enum :default "ActorDestroyed"))
  (if (Utilities|Enum|Equal(Enum) EndPlayReason "ActorDestroyed")
    (bind _asshootercharacter (Utilities|Casting|CastToShooterCharacter (Variables|Default|GetInstigator)))
    (Class|ShooterCharacter|NetSetHeadHairPercent _asshootercharacter (Variables|Default|GetHairLength) (Variables|Default|GetHairstyle))
    (Class|ShooterCharacter|NetSetFacialHairPercent _asshootercharacter (Variables|Default|GetBeardLength) (Variables|Default|GetBeardStyle))))

(event EventBeginPlay
  (Utilities|FlowControl|Delay 0.2)
  (Networking|SwitchHasAuthority
    (:Authority
      (bind _asshootercharacter (Utilities|Casting|CastToShooterCharacter (Variables|Default|GetInstigator)))
      (Utilities|FlowControl|Sequence
        (:then_0
          (Variables|Default|SetHairstyle (Math|Conversions|ToInteger(Byte) (Variables|/Script/ShooterGame.ShooterCharacter|GetHeadHairIndex _asshootercharacter)))
          (Variables|Default|SetBeardStyle (Math|Conversions|ToInteger(Byte) (Variables|/Script/ShooterGame.ShooterCharacter|GetFacialHairIndex _asshootercharacter)))
          (Variables|Default|SetHairLength (Variables|/Script/ShooterGame.ShooterCharacter|GetPercentOfFullHeadHairGrowth _asshootercharacter))
          (Variables|Default|SetBeardLength (Variables|/Script/ShooterGame.ShooterCharacter|GetPercentOfFullFacialHairGrowth _asshootercharacter))
          (Variables|Default|SetCarryWeight (Math|Float|Floor (Class|PrimalCharacterStatusComponent|BPGetCurrentStatusValue (Variables|/Script/ShooterGame.PrimalCharacter|GetMyCharacterStatusComponent _asshootercharacter) "Weight"))))
        (:then_1
          (Class|ShooterCharacter|NetSetHeadHairPercent _asshootercharacter 1.0 2)
          (Class|ShooterCharacter|NetSetFacialHairPercent _asshootercharacter 1.0 2)
          (Class|PrimalCharacterStatusComponent|UpdatedCurrentStatusValue (Variables|/Script/ShooterGame.PrimalCharacter|GetMyCharacterStatusComponent _asshootercharacter) "Weight" 1.2e+03 false 0 false false))))))

(fn ConstructionScript)